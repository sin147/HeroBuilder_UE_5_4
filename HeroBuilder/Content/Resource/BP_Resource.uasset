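; BP_Resource is a damageable resource object that shows a health bar and announces the resource it yields when depleted.
; OnHealthChanged passes current and max health to the WB_HealthBar widget.
; OnDeath hides that bar, then fills a WB_GetResource widget with the resource type and amount and shows it.
; The Blueprint only drives these two widget components, with no health or damage logic in its graphs.
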(event `self.OnHealthChanged`
  (params (OldHealth :type "Float (single-precision)") (NewHealth :type "Float (single-precision)") (MaxHealthValue :type "Float (single-precision)") (Attacker :type "Actor Object Reference"))
  (bind _aswb_health_bar (cast `/Game/UI/WB_HealthBar` (`WidgetComponent.GetWidget` (`self.HealthBarWidget`))))
  (`/Game/UI/WB_HealthBar.SetHealthRate` _aswb_health_bar NewHealth MaxHealthValue))

(event `self.OnDeath`
  (`|ExecutionSequence`
    (:`then_0`
      (bind _aswb_health_bar (cast `/Game/UI/WB_HealthBar` (`WidgetComponent.GetWidget` (`self.HealthBarWidget`))))
      (`/Game/UI/WB_HealthBar.CE_HiddeHealthBar` _aswb_health_bar))
    (:`then_1`
      (bind _aswb_get_resource (cast `/Game/UI/WB_GetResource` (`WidgetComponent.GetWidget` (`self.GetSourceWodget`))))
      (`/Game/UI/WB_GetResource.Init` _aswb_get_resource (`self.GetResourceType`) (`self.GetResourceAmount`))
      (`/Game/UI/WB_GetResource.CE_Show` _aswb_get_resource))))

(fn `UserConstructionScript`)